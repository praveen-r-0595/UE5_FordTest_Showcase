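; Actor component that builds dynamic material instances from a JSON description, loaded via VaRest at BeginPlay.
; UpdateMaterialFromJsonFile branches on the "type" field, creating and returning either a simple color material (the default) or a textured PBR one.
; JSON values drive the scalar and color parameters, while textures come from component variables.
; The emission texture is written to the "AoRM" parameter, overwriting the AoRM map.
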(event `self.ReceiveBeginPlay`
  (bind _returnvalue (`VaRestSubsystem.LoadJsonFromFile` (subsystem `VaRestSubsystem`) (`self.jsonPath`) false))
  (set `self.jsonData` _returnvalue))

(fn `UpdateMaterialFromJsonFile`
  (returns (MaterialToUpdate :type "MaterialInstanceDynamic Object Reference"))
  (bind _jsondata (`self.jsonData`))
  (bind _materialtoupdate (`self.MaterialToUpdate`))
  (bind _materialtoupdate_2 (`self.MaterialToUpdate`))
  (bind _materialtoupdate_3 (`self.MaterialToUpdate`))
  (bind _materialtoupdate_4 (`self.MaterialToUpdate`))
  (bind _jsondata_2 (`self.jsonData`))
  (bind _returnvalue (`VaRestJsonObject.GetObjectField` _jsondata_2 "albedoparams"))
  (bind _returnvalue_2 (`VaRestJsonObject.GetObjectField` _jsondata_2 "aormparams"))
  ;[0.15 0.15 0.15 0.5 36] Material Type Check From Json File
  (switch `string` (`VaRestJsonObject.GetStringField` (`self.jsonData`) "type")
    (:`Default`
      ;[0.15 0.15 0.15 0.5 36] Simple Color Material
      (bind _returnvalue_3 (`KismetMaterialLibrary.CreateDynamicMaterialInstance` (`self.MM_SimpleColor`) "simpleColorMaterial" :!label _label))
      (set `self.MaterialToUpdate` _returnvalue_3)
      (`|ExecutionSequence`
        (:`then_0`
          (`MaterialInstanceDynamic.SetVectorParameterValue` _materialtoupdate_4 "Color" (`KismetMathLibrary.Conv_DoubleToLinearColor` (`VaRestJsonObject.GetNumberField` _jsondata "color"))))
        (:`then_1`
          (`MaterialInstanceDynamic.SetScalarParameterValue` _materialtoupdate_4 "Roughness" (`VaRestJsonObject.GetNumberField` _jsondata "roughness")))
        (:`then_2`
          (if (`VaRestJsonObject.GetBoolField` _jsondata "metallic")
            (`MaterialInstanceDynamic.SetScalarParameterValue` _materialtoupdate_4 "Metallic" 1.0)
            (else
              (`MaterialInstanceDynamic.SetScalarParameterValue` _materialtoupdate_4 "Metallic" 0.0))))
        (:`then_3`
          (return (`self.MaterialToUpdate`)))))
    (:`simpleColor`
      (goto _label))
    (:`textures`
      ;[0.15 0.15 0.15 0.5 36] Textures Based Material
      (bind _returnvalue_4 (`KismetMaterialLibrary.CreateDynamicMaterialInstance` (`self.MM_Textures`) "TexturesMaterial"))
      (bind _output_get (set `self.MaterialToUpdate` _returnvalue_4))
      (`|ExecutionSequence`
        (:`then_0`
          (`MaterialInstanceDynamic.SetTextureParameterValue` _output_get "Albedo" (`self.pbr_Albedo`))
          (`MaterialInstanceDynamic.SetScalarParameterValue` _materialtoupdate "Brightness" (`VaRestJsonObject.GetNumberField` _returnvalue "brightness"))
          (`MaterialInstanceDynamic.SetScalarParameterValue` _materialtoupdate "Contrast" (`VaRestJsonObject.GetNumberField` _returnvalue "contrast"))
          (`MaterialInstanceDynamic.SetScalarParameterValue` _materialtoupdate "Tint" (`VaRestJsonObject.GetNumberField` _returnvalue "tint")))
        (:`then_1`
          (`MaterialInstanceDynamic.SetTextureParameterValue` _materialtoupdate_2 "Normal" (`self.pbr_Normal`))
          (`MaterialInstanceDynamic.SetScalarParameterValue` (`self.MaterialToUpdate`) "NormalIntensity" (`VaRestJsonObject.GetNumberField` (`VaRestJsonObject.GetObjectField` _jsondata_2 "normalparams") "normalintensity")))
        (:`then_2`
          (`MaterialInstanceDynamic.SetTextureParameterValue` (`self.MaterialToUpdate`) "AoRM" (`self.pbr_AoRM`))
          (`MaterialInstanceDynamic.SetScalarParameterValue` _materialtoupdate_3 "RoughnessIntensity" (`VaRestJsonObject.GetNumberField` _returnvalue_2 "roughness"))
          (`MaterialInstanceDynamic.SetScalarParameterValue` _materialtoupdate_3 "Specular" (`VaRestJsonObject.GetNumberField` _returnvalue_2 "specular")))
        (:`then_3`
          (`MaterialInstanceDynamic.SetTextureParameterValue` (`self.MaterialToUpdate`) "AoRM" (`self.pbr_Emission`))
          (`MaterialInstanceDynamic.SetScalarParameterValue` (`self.MaterialToUpdate`) "EmissionIntensity" (`VaRestJsonObject.GetNumberField` (`VaRestJsonObject.GetObjectField` _jsondata_2 "aormparams") "emitintensity")))
        (:`then_4`
          (`MaterialInstanceDynamic.SetScalarParameterValue` _materialtoupdate_2 "Tiling" (`VaRestJsonObject.GetNumberField` _jsondata_2 "tiling")))
        (:`then_5`
          (return (`self.MaterialToUpdate`)))))))